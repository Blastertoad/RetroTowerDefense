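; GlobalFunctions is a set of shared getters for global settings in the tower defence game.
; Each function casts the game instance to GI_TowerDefence and returns one stored value: grid scale, SFX volume or UI volume.
; The getters only read from the game instance and return no stored value if the cast fails.
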(fn `Get Grid Scale`
  (returns (GridScale :type "Float (double-precision)"))
  (bind _asgi_tower_defence (cast `/Game/Blueprint/ModesAndInstance/GI_TowerDefence` (`GameplayStatics.GetGameInstance` null)))
  (return (`/Game/Blueprint/ModesAndInstance/GI_TowerDefence.GridScale` _asgi_tower_defence)))

(fn `Get Grid Volume SFX`
  (returns (GridScale :type "Float (double-precision)"))
  (bind _asgi_tower_defence (cast `/Game/Blueprint/ModesAndInstance/GI_TowerDefence` (`GameplayStatics.GetGameInstance` null)))
  (return (`/Game/Blueprint/ModesAndInstance/GI_TowerDefence.VolumeSFX` _asgi_tower_defence)))

(fn `Get Grid Volume UI`
  (returns (GridScale :type "Float (double-precision)"))
  (bind _asgi_tower_defence (cast `/Game/Blueprint/ModesAndInstance/GI_TowerDefence` (`GameplayStatics.GetGameInstance` null)))
  (return (`/Game/Blueprint/ModesAndInstance/GI_TowerDefence.VolumeUI` _asgi_tower_defence)))