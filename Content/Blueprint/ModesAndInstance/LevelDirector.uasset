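; LevelDirector runs a tower defence level's flow, from intro story screen through enemy waves to loading the next level or menu.
; BeginPlay starts music that follows the game instance's volume, then shows the HUD and story pane, using end lines when EndGame is set.
; StartGame possesses a tactical pawn spawned above the goals' average location and starts the level.
; SpawnWave recursively spawns delayed waves at index-matched entry points, then flags LastWave on the game mode.
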(event `Show story Screen`
  (if (`self.EndGame`) :!label _label
    (set `self.StoryLines` (`self.EndLines`)))
  (bind _returnvalue (`|CreateWidget` "/Game/Widgets/UMG_Hud.UMG_Hud_C" (`GameplayStatics.GetPlayerController` 0)))
  (`UserWidget.AddToViewport` _returnvalue 0)
  (bind _returnvalue_2 (`|CreateWidget` "/Game/Widgets/Story/UMG_StoryPane.UMG_StoryPane_C" (`GameplayStatics.GetPlayerController` 0)))
  (`UserWidget.AddToViewport` _returnvalue_2 0))

(event `self.ReceiveBeginPlay`
  ;[1 1 1] Music
  (bind _asgi_tower_defence (cast `/Game/Blueprint/ModesAndInstance/GI_TowerDefence` (`GameplayStatics.GetGameInstance`)))
  (add `/Game/Blueprint/ModesAndInstance/GI_TowerDefence.MusicUpdated` _asgi_tower_defence (delegate `Change music volume`))
  (bind _returnvalue (`GameplayStatics.SpawnSound2D` (`self.LevelMusic`) (`/Game/Blueprint/ModesAndInstance/GI_TowerDefence.VolumeMusic` _asgi_tower_defence) 1.0 0.0 null true))
  (set `self.Music` _returnvalue)
  (goto _label))

(event `Change music volume`
  ;[1 1 1] Music
  (bind _asgi_tower_defence (cast `/Game/Blueprint/ModesAndInstance/GI_TowerDefence` (`GameplayStatics.GetGameInstance`)))
  (`AudioComponent.SetVolumeMultiplier` (`self.Music`) (`/Game/Blueprint/ModesAndInstance/GI_TowerDefence.VolumeMusic` _asgi_tower_defence)))

(event `Spawn Wave`
  (bind (_returnvalue_location _returnvalue_rotation) (`KismetMathLibrary.BreakTransform` (`self.GetTransform` (`self.EntryPoint`))))
  (bind (_delay _entryindex _composition) (break `/Game/Blueprint/Enemies/Struct_Wave` (`|GetArrayItem` (`self.Waves`) (`self.WaveIndex`))))
  ;[1 1 1] Find entry point for wave to spawn at
  (`KismetSystemLibrary.Delay` _delay)
  (bind _outactors (`GameplayStatics.GetAllActorsOfClass` "/Game/Blueprint/Enemies/EntryPoint.EntryPoint_C"))
  (for _array_element _outactors
    (if (== (`/Game/Blueprint/Enemies/EntryPoint.EntryPoint Index` _array_element) _entryindex)
      (set `self.EntryPoint` _array_element)
      (break)))
  ;[1 1 1] Spawn each enemy in wave
  (for _array_element_2 _composition
    (`|SpawnActorFromClass` _array_element_2 (`KismetMathLibrary.MakeTransform` (+ _returnvalue_location (0.0 0.0 500.0)) _returnvalue_rotation (`KismetMathLibrary.Conv_DoubleToVector` 0.9)) "AdjustIfPossibleButAlwaysSpawn" "OverrideRootScale" null null))
  ;[1 1 1] Progress wave number. If out of range set last wave on game mode
  (bind _output_get (set `self.WaveIndex` (+ (`self.WaveIndex`) 1)))
  (if (`KismetArrayLibrary.Array_IsValidIndex` (`self.Waves`) _output_get)
    (`self.Spawn Wave`)
    (else
      (bind _asgm_tower_defence (cast `/Game/Blueprint/ModesAndInstance/GM_TowerDefence` (`GameplayStatics.GetGameMode`)))
      (set `/Game/Blueprint/ModesAndInstance/GM_TowerDefence.Last Wave` true _asgm_tower_defence))))

(event `Start Game`
  (bind _nextlevel (`self.NextLevel`))
  (if (`self.EndGame`)
    (if (== _nextlevel "None")
      (`GameplayStatics.OpenLevel` "Map_Menu")
      (else
        (`GameplayStatics.OpenLevel` _nextlevel)))
    (else
      (`KismetSystemLibrary.Delay` 0.1)
      ;[1 1 1] Spawn between all goals
      (bind _outactors (`GameplayStatics.GetAllActorsOfClass` "/Game/Blueprint/Player/Class_Goal.Class_Goal_C"))
      (for _array_element _outactors
        (set `self.Location` (+ (`self.Location`) (`self.K2_GetActorLocation` _array_element))))
      (bind _returnvalue (`|SpawnActorFromClass` "/Game/Blueprint/Player/P_Tactical.P_Tactical_C" (`KismetMathLibrary.MakeTransform` (+ (/ (`self.Location`) (`KismetArrayLibrary.Array_Length` _outactors)) (0.0 0.0 2000.0))) "Undefined" "OverrideRootScale" null null))
      (`Controller.Possess` (`GameplayStatics.GetPlayerController` 0) _returnvalue)
      (bind _asgm_tower_defence (cast `/Game/Blueprint/ModesAndInstance/GM_TowerDefence` (`GameplayStatics.GetGameMode`)))
      (`/Game/Blueprint/ModesAndInstance/GM_TowerDefence.Level Start` _asgm_tower_defence)
      (`self.Spawn Wave`))))

(fn `UserConstructionScript`)