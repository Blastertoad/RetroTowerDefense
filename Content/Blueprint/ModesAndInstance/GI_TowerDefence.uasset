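; Game instance for the tower defence game that persists audio settings and player progress through a single save slot.
; On init it loads the save, copies the SFX, UI and music volumes and the level into its variables, then broadcasts MusicUpdated.
; SaveSettings writes only the volumes and rebroadcasts, while SaveGame also stores the passed level and credits.
; If no valid save loads, initialisation stops without creating one.
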(event `self.ReceiveInit`
  (`self.Load Game`))

(event `Load Game`
  (bind _returnvalue (`GameplayStatics.LoadGameFromSlot` "Save"))
  (bind _assave_tower_game (cast `/Game/Blueprint/ModesAndInstance/Save_TowerGame` _returnvalue))
  (bind _output_get (set `self.Save` _assave_tower_game))
  (set `self.VolumeSFX` (`/Game/Blueprint/ModesAndInstance/Save_TowerGame.VolumeSFX` _output_get))
  (set `self.VolumeUI` (`/Game/Blueprint/ModesAndInstance/Save_TowerGame.VolumeUI` _output_get))
  (set `self.VolumeMusic` (`/Game/Blueprint/ModesAndInstance/Save_TowerGame.VolumeMusic` _output_get))
  (set `self.Level` (`/Game/Blueprint/ModesAndInstance/Save_TowerGame.Level` _output_get))
  (`self.MusicUpdated` :!label _label))

(event `Save Settings`
  (bind _save (`self.Save`))
  (set `/Game/Blueprint/ModesAndInstance/Save_TowerGame.VolumeSFX` (`self.VolumeSFX`) _save)
  (set `/Game/Blueprint/ModesAndInstance/Save_TowerGame.VolumeUI` (`self.VolumeUI`) _save)
  (set `/Game/Blueprint/ModesAndInstance/Save_TowerGame.VolumeMusic` (`self.VolumeMusic`) _save)
  (`GameplayStatics.SaveGameToSlot` (`self.Save`) "Save")
  (goto _label))

(event `SaveGame`
  (params (Level :type Name) (Credits :type Integer))
  (bind _save (`self.Save`))
  (set `/Game/Blueprint/ModesAndInstance/Save_TowerGame.VolumeSFX` (`self.VolumeSFX`) _save)
  (set `/Game/Blueprint/ModesAndInstance/Save_TowerGame.VolumeUI` (`self.VolumeUI`) _save)
  (set `/Game/Blueprint/ModesAndInstance/Save_TowerGame.VolumeMusic` (`self.VolumeMusic`) _save)
  (set `/Game/Blueprint/ModesAndInstance/Save_TowerGame.Level` Level _save)
  (set `/Game/Blueprint/ModesAndInstance/Save_TowerGame.Credits` Credits _save)
  (`GameplayStatics.SaveGameToSlot` (`self.Save`) "Save"))