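; Tower defence game mode that holds the player's credits and decides when a level is won or lost.
; EnemyDeath adds the kill reward and, on the last wave, fires LevelEnd if no Char_Enemy actors remain.
; GoalLost fires GameOver once no goal actors remain.
; LevelStart and GameOver are empty events, and LevelEnd only prints a message.
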(event `Level Start`)

(event `Level End`
  (`KismetSystemLibrary.PrintString` "Level Over"))

(event `GameOver`)

(fn `EnemyDeath`
  (params (Credits :type Integer))
  ;[1 1 1] Collect reward for destoying enemy, if last wave check if there are enemies left in play, if not trigger level end.
  (set `self.Credits` (+ Credits (`self.Credits`)))
  (if (`self.Last Wave`)
    (bind _outactors (`GameplayStatics.GetAllActorsOfClass` "/Game/Blueprint/Enemies/Char_Enemy.Char_Enemy_C"))
    (if (<= (`KismetArrayLibrary.Array_Length` _outactors) 0)
      (`self.Level End`))))

(fn `Goal Lost`
  (bind _outactors (`GameplayStatics.GetAllActorsOfClass` "/Game/Blueprint/Player/Class_Goal.Class_Goal_C"))
  (if (<= (`KismetArrayLibrary.Array_Length` _outactors) 0)
    (`self.GameOver`)))

(fn `UserConstructionScript`)