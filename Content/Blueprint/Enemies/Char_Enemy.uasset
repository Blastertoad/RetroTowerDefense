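; Tower defence enemy character that damages player-owned targets and reports its death reward to GM_TowerDefence.
; A looping fire-rate timer damages the current target, set and cleared by AttackTrigger overlaps filtered on I_PlayerOwned and Visibility blocking.
; SelectGoal writes the nearest qualifying goal actor to the AI Blackboard, but nothing live here calls it.
; Incoming damage reduces Health and notifies the game mode at zero or below.
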(event `self.ReceiveBeginPlay`
  (`KismetSystemLibrary.K2_SetTimerDelegate` (delegate `AttackLoop`) (`self.Fire Rate`) true))

(event `Select Goal`
  ;[1 1 1] Set ai target goal to the closest goal object
  (bind _outactors (`GameplayStatics.GetAllActorsOfClass` "/Game/Blueprint/Player/Class_Goal.Class_Goal_C"))
  (for _array_element _outactors
    (bind _returnvalue (`self.GetDistanceTo` _array_element self))
    (if (<= _returnvalue (`self.GoalDistance`))
      (set `self.GoalDistance` _returnvalue)
      (set `self.Goal` _array_element)))
  (`BlackboardComponent.SetValueAsObject` (`AIBlueprintHelperLibrary.GetBlackboard` self) "Goal" (`self.Goal`)))

(event `AttackLoop`
  (bind _target (`self.Target`))
  ;[1 1 1] If attack bool is true do damage on timer loop
  (if (`self.Attack`)
    (`/Engine/EditorBlueprintResources/StandardMacros.IsValid` _target
      (:`Is Valid`
        (`GameplayStatics.ApplyDamage` _target (`self.Damage`) null self)
        (`KismetSystemLibrary.PrintString` "Attack")))))

(event `self.AttackTrigger.OnComponentBeginOverlap`
  (params (OverlappedComponent :type "PrimitiveComponent Object Reference") (OtherActor :type "Actor Object Reference") (OtherComp :type "PrimitiveComponent Object Reference") (OtherBodyIndex :type Integer) (bFromSweep :type Boolean) (SweepResult :type "HitResult Structure (by ref)"))
  ;[1 1 1] Handle potential targets entering or leaving attack box
  (if (and (`KismetSystemLibrary.DoesImplementInterface` OtherActor "/Game/Blueprint/Player/I_PlayerOwned.I_PlayerOwned_C") (`|EnumEquality` (`PrimitiveComponent.GetCollisionResponseToChannel` OtherComp "ECC_Visibility") "ECR_Block"))
    (set `self.Target` OtherActor)
    (set `self.Attack` true)))

(event `self.AttackTrigger.OnComponentEndOverlap`
  (params (OverlappedComponent :type "PrimitiveComponent Object Reference") (OtherActor :type "Actor Object Reference") (OtherComp :type "PrimitiveComponent Object Reference") (OtherBodyIndex :type Integer))
  ;[1 1 1] Handle potential targets entering or leaving attack box
  (if (== (`self.Target`) OtherActor)
    (set `self.Attack` false)
    (set `self.Target` null)))

(event `self.ReceiveAnyDamage`
  (params (Damage :type "Float (single-precision)") (DamageType :type "DamageType Object Reference") (InstigatedBy :type "Controller Object Reference") (DamageCauser :type "Actor Object Reference"))
  ;[1 1 1] Recieve damage, if destroyed notify gamemode
  (bind _output_get (set `self.Health` (- (`self.Health`) Damage)))
  (if (<= _output_get 0.0)
    (bind _asgm_tower_defence (cast `/Game/Blueprint/ModesAndInstance/GM_TowerDefence` (`GameplayStatics.GetGameMode`)))
    (`/Game/Blueprint/ModesAndInstance/GM_TowerDefence.EnemyDeath` _asgm_tower_defence (`self.RewardCredits`))))

(fn `UserConstructionScript`)