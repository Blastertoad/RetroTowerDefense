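; EnemyManager spawns timed waves of enemies for a tower defence game, starting at BeginPlay.
; Each SpawnWave waits the current wave's delay, finds the EntryPoint actor matching its entry index, then spawns every class in the wave's composition just above it.
; The event calls itself to advance through the Waves array, then sets LastWave on GM_TowerDefence when none remain.
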(event `self.ReceiveBeginPlay`
  (`self.Spawn Wave`))

(event `Spawn Wave`
  (bind (_returnvalue_location _returnvalue_rotation) (`KismetMathLibrary.BreakTransform` (`self.GetTransform` (`self.EntryPoint`))))
  (bind (_delay _entryindex _composition) (break `/Game/Blueprint/Enemies/Struct_Wave` (`|GetArrayItem` (`self.Waves`) (`self.WaveIndex`))))
  ;[1 1 1] Find entry point for wave to spawn at
  (`KismetSystemLibrary.Delay` _delay)
  (bind _outactors (`GameplayStatics.GetAllActorsOfClass` "/Game/Blueprint/Enemies/EntryPoint.EntryPoint_C"))
  (for _array_element _outactors
    (if (== (`/Game/Blueprint/Enemies/EntryPoint.EntryPoint Index` _array_element) _entryindex)
      (set `self.EntryPoint` _array_element)
      (break)))
  ;[1 1 1] Spawn each enemy in wave
  (for _array_element_2 _composition
    (`|SpawnActorFromClass` _array_element_2 (`KismetMathLibrary.MakeTransform` (+ _returnvalue_location (0.0 0.0 50.0)) _returnvalue_rotation) "AdjustIfPossibleButAlwaysSpawn" "OverrideRootScale" null null))
  ;[1 1 1] Progress wave number. If out of range set last wave on game mode
  (bind _output_get (set `self.WaveIndex` (+ (`self.WaveIndex`) 1)))
  (if (`KismetArrayLibrary.Array_IsValidIndex` (`self.Waves`) _output_get)
    (`self.Spawn Wave`)
    (else
      (bind _asgm_tower_defence (cast `/Game/Blueprint/ModesAndInstance/GM_TowerDefence` (`GameplayStatics.GetGameMode`)))
      (set `/Game/Blueprint/ModesAndInstance/GM_TowerDefence.Last Wave` true _asgm_tower_defence))))

(fn `UserConstructionScript`)