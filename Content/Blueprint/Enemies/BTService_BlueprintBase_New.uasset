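; Behavior tree service for enemy AI that picks the actor of a configurable class nearest to the controlled pawn as its goal.
; On each tick without a valid Goal, it scans all actors of that class, keeping the closest by distance.
; It writes the result to the GoalKey blackboard entry and prints a debug string.
; A valid Goal is kept, even if another actor becomes closer.
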(event `self.ReceiveTickAI`
  (params (OwnerController :type "AIController Object Reference") (ControlledPawn :type "Pawn Object Reference") (DeltaSeconds :type "Float (single-precision)"))
  (`/Engine/EditorBlueprintResources/StandardMacros.IsValid` (`self.Goal`)
    (:`Is Not Valid`
      (bind _outactors (`GameplayStatics.GetAllActorsOfClass` "/Game/Blueprint/Player/Class_Goal.Class_Goal_C"))
      (for (_array_element _array_index) _outactors
        (if (== _array_index 0)
          (bind _returnvalue (`Actor.GetDistanceTo` _array_element ControlledPawn))
          (set `self.GoalDistance` _returnvalue :!label _label)
          (set `self.Goal` _array_element)
          (elif (<= _returnvalue (`self.GoalDistance`))
            (goto _label))))
      (`BTFunctionLibrary.SetBlackboardValueAsObject` (`self.GoalKey`) (`self.Goal`))
      (`KismetSystemLibrary.PrintString` "goal"))))

(event `self.ReceiveActivationAI`
  (params (OwnerController :type "AIController Object Reference") (ControlledPawn :type "Pawn Object Reference")))