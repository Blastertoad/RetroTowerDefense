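; Tower defence turret pawn that aims itself under AI control or can be possessed by a player, who returns to the tactical pawn afterwards.
; A looping timer picks the enemy nearest a goal within radius-scaled ground and air collision volumes, with air targets taking priority.
; Tick steps yaw and clamped pitch toward it via dot-product side checks and flags when it enters the firing arc.
; The timed fire event is still empty.
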(event `Fire Weapons`
  (if (`self.FireWeapons`)
    _))

(event `self.ReceiveBeginPlay`
  (`KismetSystemLibrary.K2_SetTimerDelegate` (delegate `Select Target`) (`self.TargetUpdate Time`) true)
  (`KismetSystemLibrary.K2_SetTimerDelegate` (delegate `Fire Weapons`) (`self.FireRate`) true))

(event `Select Target`
  (bind _target (`self.Target`))
  ;[1 1 1] Select closest overlapping enemy to goal. Prioratize Air if air radius is valid
  (if (`self.AI_Controlled`)
    ;[1 1 1] Get nearest goal
    (bind _outactors (`GameplayStatics.GetAllActorsOfClass` "/Game/Blueprint/Player/Class_Goal.Class_Goal_C"))
    (for (_array_element _array_index) _outactors
      (if (== _array_index 0)
        (bind _returnvalue (`self.GetDistanceTo` _array_element self))
        (set `self.GoalDistance` _returnvalue)
        (set `self.Goal` _array_element)
        (elif (<= _returnvalue (`self.TargetDistance`))
          (set `self.GoalDistance` _returnvalue)
          (set `self.Goal` _array_element))))
    (for (_array_element_2 _array_index_2) (`PrimitiveComponent.GetOverlappingActors` (`self.GroundCollision`) "/Game/Blueprint/Enemies/Char_Enemy.Char_Enemy_C")
      (if (== _array_index_2 0)
        (bind _returnvalue_2 (`self.GetDistanceTo` _array_element_2 (`self.Goal`)))
        (set `self.TargetDistance` _returnvalue_2)
        (set `self.Target` _array_element_2)
        (elif (<= _returnvalue_2 (`self.TargetDistance`))
          (set `self.TargetDistance` _returnvalue_2)
          (set `self.Target` _array_element_2))))
    (if (>= (`self.AirRadius`) 1.0)
      (for (_array_element_3 _array_index_3) (`PrimitiveComponent.GetOverlappingActors` (`self.AirCollision`) "/Game/Blueprint/Enemies/Char_Enemy.Char_Enemy_C")
        (if (== _array_index_3 0)
          (bind _returnvalue_3 (`self.GetDistanceTo` _array_element_3 (`self.Goal`)))
          (set `self.TargetDistance` _returnvalue_3)
          (set `self.Target` _array_element_3)
          (elif (<= _returnvalue_3 (`self.TargetDistance`))
            (set `self.TargetDistance` _returnvalue_3)
            (set `self.Target` _array_element_3))))
      ;[1 1 1] If target is out or ai range clear target
      (if (not (or (`KismetArrayLibrary.Array_Contains` (`PrimitiveComponent.GetOverlappingActors` (`self.GroundCollision`) "/Game/Blueprint/Enemies/Char_Enemy.Char_Enemy_C") _target) (`KismetArrayLibrary.Array_Contains` (`PrimitiveComponent.GetOverlappingActors` (`self.AirCollision`) "/Game/Blueprint/Enemies/Char_Enemy.Char_Enemy_C") _target)))
        (set `self.Target` null)))))

(event `self.ReceiveTick`
  (params (DeltaSeconds :type "Float (single-precision)"))
  (bind _returnvalue (`GameplayStatics.GetWorldDeltaSeconds`))
  (bind _target (`self.Target`))
  (bind _yaw (`self.Yaw`))
  (bind _pitch (`self.Pitch`))
  (bind _returnvalue_2 (`SceneComponent.K2_GetComponentRotation` _yaw))
  (bind _returnvalue_3 (`SceneComponent.K2_GetComponentRotation` _pitch))
  ;[1 1 1] Is enemy in firing arc
  (if (`self.AI_Controlled`)
    (`/Engine/EditorBlueprintResources/StandardMacros.IsValid` _target
      (:`Is Valid`
        (if (<= (`KismetMathLibrary.DegAcos` (`KismetMathLibrary.Dot_VectorVector` (`SceneComponent.GetForwardVector` (`self.Pitch`)) (`KismetMathLibrary.GetForwardVector` (`KismetMathLibrary.FindLookAtRotation` (`self.K2_GetActorLocation` self) (`self.K2_GetActorLocation` _target))))) (/ (`self.FiringArc`) 2.0))
          (set `self.FireWeapons` true)
          (else
            (set `self.FireWeapons` false)))
        ;[1 1 1] Rotate turret to face enemy
        (`SceneComponent.K2_SetWorldRotation` _pitch (`KismetMathLibrary.RInterpTo` _returnvalue_3 (`KismetMathLibrary.MakeRotator` (.roll _returnvalue_3) (`KismetMathLibrary.ClampAngle` (+ (.pitch _returnvalue_3) (* (`self.TurnRate`) (select `bool` (<= (`KismetMathLibrary.DegAcos` (`KismetMathLibrary.Dot_VectorVector` (`SceneComponent.GetUpVector` (`self.Pitch`)) (`KismetMathLibrary.GetForwardVector` (`KismetMathLibrary.FindLookAtRotation` (`self.K2_GetActorLocation` self) (`self.K2_GetActorLocation` (`self.Target`)))))) 90.0) :`false` -1.0 :`true` 1.0 :!type "Float (single-precision)") (`GameplayStatics.GetWorldDeltaSeconds`))) -80.0 80.0) (.yaw _returnvalue_3)) _returnvalue 100.0) false false)
        (`SceneComponent.K2_SetWorldRotation` _yaw (`KismetMathLibrary.RInterpTo` _returnvalue_2 (`KismetMathLibrary.MakeRotator` (.roll _returnvalue_2) (.pitch _returnvalue_2) (+ (.yaw _returnvalue_2) (* (`self.TurnRate`) (select `bool` (<= (`KismetMathLibrary.DegAcos` (`KismetMathLibrary.Dot_VectorVector` (`SceneComponent.GetRightVector` (`self.Yaw`)) (`KismetMathLibrary.GetForwardVector` (`KismetMathLibrary.FindLookAtRotation` (`self.K2_GetActorLocation` self) (`self.K2_GetActorLocation` (`self.Target`)))))) 90.0) :`false` -1.0 :`true` 1.0 :!type "Float (single-precision)") (`GameplayStatics.GetWorldDeltaSeconds`)))) _returnvalue 100.0) false false)))))

(fn `Possess Turret`
  (params (NewParam :type "PlayerController Object Reference"))
  (`Controller.Possess` NewParam self)
  (set `self.AI_Controlled` false))

(fn `Un-Possess Turret`
  (bind _aspc_tower_defence (cast `/Game/Blueprint/Player/PC_TowerDefence` (`self.GetController`)))
  (`Controller.Possess` _aspc_tower_defence (`/Game/Blueprint/Player/PC_TowerDefence.Pawn Tactical` _aspc_tower_defence))
  (set `self.AI_Controlled` true))

(fn `UserConstructionScript`
  (bind _groundcollision (`self.GroundCollision`))
  (bind _returnvalue (`SceneComponent.K2_GetComponentToWorld` _groundcollision))
  (bind _returnvalue_2 (* (`self.GroundRadius`) 2.0))
  (`SceneComponent.SetWorldScale3D` (`self.AirCollision`) (`KismetMathLibrary.Conv_DoubleToVector` (* (`self.AirRadius`) 2.0)))
  (`SceneComponent.K2_SetWorldTransform` _groundcollision (`KismetMathLibrary.MakeTransform` (`KismetMathLibrary.MakeVector` (.x (.location _returnvalue)) (.y (.location _returnvalue))) (.rotation _returnvalue) (`KismetMathLibrary.MakeVector` _returnvalue_2 _returnvalue_2 1.5)) false false))