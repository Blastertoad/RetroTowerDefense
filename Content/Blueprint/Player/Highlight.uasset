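; Highlight is an actor that animates the scale of a Plane until a sphere trace detects a hit at its location.
; BeginPlay runs a short sphere trace on a custom channel and destroys the actor on a hit.
; Otherwise a timeline drives the plane's scale, printing the value each update, and loops back to the trace when finished, so detection happens only between animation cycles.
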(event `self.ReceiveBeginPlay`
  (bind _returnvalue (`self.K2_GetActorLocation`))
  (bind (_outhit _returnvalue_2) (`KismetSystemLibrary.SphereTraceSingle` _returnvalue (+ _returnvalue (0.0 0.0 1.0)) 20.0 "TraceTypeQuery3" :!label _label))
  (if _returnvalue_2
    (`self.K2_DestroyActor`)
    (else
      (bind (_direction _newtrack_0) (`Timeline|Timeline_0` :!via `PlayFromStart`)
        (:`Update`
          (bind _returnvalue_3 (`KismetMathLibrary.Conv_DoubleToVector` _newtrack_0))
          (`SceneComponent.SetWorldScale3D` (`self.Plane`) _returnvalue_3)
          (`KismetSystemLibrary.PrintString` (`KismetStringLibrary.Conv_VectorToString` _returnvalue_3)))
        (:`Finished`
          (goto _label))))))

(fn `UserConstructionScript`)