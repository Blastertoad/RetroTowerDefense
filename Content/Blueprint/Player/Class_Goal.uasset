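; Goal actor for a tower defence mode that the game treats as lost when its health runs out.
; Tick spins four ring components at fixed, differing speeds and directions for a constant decorative motion.
; Any damage reduces and prints Health; at zero it plays an explosion sound scaled by the grid SFX volume, destroys itself and notifies GM_TowerDefence through GoalLost.
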(event `self.ReceiveTick`
  (params (DeltaSeconds :type "Float (single-precision)"))
  (`SceneComponent.K2_AddLocalRotation` (`self.Ring1`) (struct :`Yaw` 0.2) false false)
  (`SceneComponent.K2_AddLocalRotation` (`self.Ring2`) (struct :`Yaw` -0.2) false false)
  (`SceneComponent.K2_AddLocalRotation` (`self.Ring3`) (struct :`Yaw` 0.5) false false)
  (`SceneComponent.K2_AddLocalRotation` (`self.Ring4`) (struct :`Yaw` -0.2) false false))

(event `self.ReceiveAnyDamage`
  (params (Damage :type "Float (single-precision)") (DamageType :type "DamageType Object Reference") (InstigatedBy :type "Controller Object Reference") (DamageCauser :type "Actor Object Reference"))
  (bind _output_get (set `self.Health` (- (`self.Health`) Damage)))
  (`KismetSystemLibrary.PrintString` (`KismetStringLibrary.Conv_DoubleToString` _output_get))
  (if (<= _output_get 0.0)
    (bind _gridscale (`/Game/Blueprint/ModesAndInstance/GlobalFunctions.Get Grid Volume SFX`))
    (`GameplayStatics.SpawnSoundAttached` "/Game/Retro_8Bit_Sounds/Explosion/Cues/retro_explosion_deep_18_Cue.retro_explosion_deep_18_Cue" (`self.Base`) "None" (0.0 0.0 0.0) (struct) "KeepRelativeOffset" false (+ _gridscale 0.3) 1.0 0.0 "/Game/Blueprint/Sound/NewSoundAttenuation.NewSoundAttenuation" null)
    (`self.K2_DestroyActor`)
    (bind _asgm_tower_defence (cast `/Game/Blueprint/ModesAndInstance/GM_TowerDefence` (`GameplayStatics.GetGameMode`)))
    (`/Game/Blueprint/ModesAndInstance/GM_TowerDefence.Goal Lost` _asgm_tower_defence)))

(fn `UserConstructionScript`)