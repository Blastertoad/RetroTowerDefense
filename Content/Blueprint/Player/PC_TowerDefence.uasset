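; Player controller for the tower defence game that handles pausing through the Back input, ignored while controlling a turret.
; A FlipFlop alternates presses between pausing with the UMG_Paused widget and arming a resume.
; On the resume press, releasing Back unpauses and removes the widget.
; A one-second Delay into a Gate, closed on release, is wired as hold-to-quit to Map_Menu.
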(event `InputAction|Back` :consume false :paused true
  (params (Key :type "Key Structure"))
  (:`Pressed`
    (cast `/Game/Blueprint/Player/Turrets/Class_Turret` (`self.K2_GetPawn`)
      (:`CastFailed`
        (`/Engine/EditorBlueprintResources/StandardMacros.FlipFlop`
          (:`A`
            (`GameplayStatics.SetGamePaused` true)
            (bind _returnvalue (`|CreateWidget` "/Game/Widgets/UMG_Paused.UMG_Paused_C"))
            (`UserWidget.AddToViewport` _returnvalue 0)
            (set `self.Paused` true))
          (:`B`
            (`|ExecutionSequence`
              (:`then_0`
                (`KismetSystemLibrary.Delay` 1.0)
                (`/Engine/EditorBlueprintResources/StandardMacros.Gate` true :!label _label
                  (:`Exit`
                    (`GameplayStatics.OpenLevel` "Map_Menu"))))
              (:`then_1`
                (goto _label :!via `Open`))
              (:`then_2`
                (set `self.Paused` false))))))))
  (:`Released`
    (`|ExecutionSequence`
      (:`then_0`
        (goto _label :!via `Close`))
      (:`then_1`
        (if (not (`self.Paused`))
          (`GameplayStatics.SetGamePaused` false)
          (bind _foundwidgets (`WidgetBlueprintLibrary.GetAllWidgetsOfClass` "/Game/Widgets/UMG_Paused.UMG_Paused_C"))
          (for _array_element _foundwidgets
            (`Widget.RemoveFromParent` _array_element)))))))

(fn `UserConstructionScript`)